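; Blueprint interface for the hover car system, declaring the calls other objects use to talk to a hover vehicle without knowing its class.
; It covers applying linear and angular forces and getting the PhysX mesh and speed.
; It also reads and sets stick-to-surface and ignore-stick states, with a flag for changes made by volumes, and exposes boost toggling and numbered camera switching.
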(fn AddForce
  (params (Force :type Vector) (Location :type Vector) (SMComponent :type Static%20Mesh%20Component%20Object%20Reference)))

(fn GetPhysxMeshReference
  (return 0))

(fn GetSticktoSurface
  (return false))

(fn GetIgnoreStick
  (return false))

(fn GetSpeed
  (return 0.0))

(fn SetSticktoSurface
  (params (StickToSurface :type Boolean)))

(fn SetIgnoreStick
  (params (IgnoreStickToSurface :type Boolean) (SetByVolume :type Boolean)))

(fn ActivateBoost)

(fn DeactivateBoost)

(fn SwitchCamera
  (params (CameraNumber :type Integer))
  (return))

(fn AddAngularForce
  (params (ForceVector :type Vector) (Force :type Float%20%28double-precision%29) (Multiplier :type Float%20%28double-precision%29))
  (return))